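; BP_Car is a player-controlled car driven through a vehicle movement component.
; MoveForward and MoveRight axis inputs feed throttle and steering directly, while Mouse X and Y add relative yaw and pitch to the spring arm to orbit the view, with no clamping in the graph.
; Handbrake on and off calls exist but no event triggers them.
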(event Input|ActionEvents|InputActionJump
  (params (Key :type Key%20Structure)))

(event Input|AxisEvents|InputAxisMouseXInput
  (params (AxisValue :type Float%20%28single-precision%29))
  ;[1 1 1] Mouse
  (Transformation|AddRelativeRotation (Variables|Default|GetSpringArm) (Math|Rotator|MakeRotator 0.0 0.0 AxisValue) false false))

(event Input|AxisEvents|InputAxisMouseYInput
  (params (AxisValue :type Float%20%28single-precision%29))
  ;[1 1 1] Mouse
  (Transformation|AddRelativeRotation (Variables|Default|GetSpringArm) (Math|Rotator|MakeRotator 0.0 AxisValue 0.0) false false))

(event Input|AxisEvents|InputAxisMoveForward
  (params (AxisValue :type Float%20%28single-precision%29))
  (Class|WheeledVehicleMovementComponent|SetThrottleInput (Variables|Default|GetVehicleMovement) AxisValue))

(event Input|AxisEvents|InputAxisMoveRight
  (params (AxisValue :type Float%20%28single-precision%29))
  (Class|WheeledVehicleMovementComponent|SetSteeringInput (Variables|Default|GetVehicleMovement) AxisValue))

(fn ConstructionScript)