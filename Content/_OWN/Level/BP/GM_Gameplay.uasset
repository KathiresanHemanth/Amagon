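; Gameplay game mode that handles players joining and leaving a multiplayer session.
; On authority, PostLogin records each controller, spawns and possesses a BP_Char_Gameplay at a player start named by join index, and creates a match window if missing.
; Logout calls the game instance's session teardown, removes the controller, and rebroadcasts the current/max player count.
; Alternating Team A/B assignment exists but is disconnected.
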(event Custom|Update%20players
  ;[1 1 1] Update Player for Auto match
  (Utilities|FlowControl|Delay 0.6)
  (bind _asmainmenu_game_instance (Utilities|Casting|CastToMainmenuGameInstance (Game|GetGameInstance)))
  (for _array_element (Variables|Default|GetAll%20Player%20Controllers)
    (bind _aspc_gameplay (Utilities|Casting|CastToPC_Gameplay _array_element))
    (Default|UpdatePlayerCount _aspc_gameplay (Utilities|String|Append (Utilities|String|ToString(Integer) (Utilities|Array|Length (Variables|Default|GetAll%20Player%20Controllers))) "/" (Utilities|String|ToString(Integer) (Variables|/Game/_OWN/UI/Mainmenu_UI/BP/MainmenuGameInstance.MainmenuGameInstance_C|GetV%20Max%20Players _asmainmenu_game_instance))))))

(event Custom|Spawn%20Player
  (params (Player :type Controller%20Object%20Reference) (Cast%20Ref :type PC%20Gameplay%20Object%20Reference))
  ;[1 1 1] Spawn Player
  (bind _returnvalue (Game|SpawnActorfromClass "/Game/_OWN/Character/Char_BP/Gameplay/BP_Char_Gameplay.BP_Char_Gameplay_C" (Transformation|GetActorTransform (Class|GameModeBase|FindPlayerStart Player (Utilities|String|ToString(Integer) (- (Utilities|Array|Length (Variables|Default|GetAll%20Player%20Controllers)) 1)))) "Undefined" Player 0))
  (Pawn|Possess Player _returnvalue)
  (bind _asgs_gameplay (Utilities|Casting|CastToGS_Gameplay (Game|GetGameState)))
  (Variables|Default|SetAs%20Gs%20Gameplay _asgs_gameplay))

(event EventPostLogin
  (params (NewPlayer :type Player%20Controller%20Object%20Reference))
  (Networking|SwitchHasAuthority
    (:Authority
      (bind _aspc_gameplay (Utilities|Casting|CastToPC_Gameplay NewPlayer))
      (Utilities|Array|Add (Variables|Default|GetAll%20Player%20Controllers) _aspc_gameplay)
      (CallFunction|SpawnPlayer _aspc_gameplay _aspc_gameplay)
      (Utilities|IsValid (Variables|/Game/_OWN/Level/BP/PC_Gameplay.PC_Gameplay_C|GetW/B%20Match%20Stats _aspc_gameplay)
        (:Is%20Not%20Valid
          (Default|CreateMatchWindowServer _aspc_gameplay NewPlayer)
          (CallFunction|UpdatePlayers))))))

(event EventOnLogout
  (params (ExitingController :type Controller%20Object%20Reference))
  ;[1 1 1] ON Logout , Destroy session
  (bind _aspc_gameplay (Utilities|Casting|CastToPC_Gameplay ExitingController))
  (Default|DestroySessionCaller (.AsMainmenu%20Game%20Instance (Utilities|Casting|CastToMainmenuGameInstance (Game|GetGameInstance))) _aspc_gameplay)
  ;[1 1 1] On Logout
  (bind (_array_element _array_index) (Utilities|Array|ForEachLoopwithBreak (Variables|Default|GetAll%20Player%20Controllers) :!label _label)
    (:LoopBody
      (if (== ExitingController _array_element)
        (goto _label Break)))
    (:Completed
      ;[1 1 1] Remove From Array
      (Utilities|Array|RemoveIndex (Variables|Default|GetAll%20Player%20Controllers) _array_index)
      (CallFunction|UpdatePlayers))))

(fn ConstructionScript)