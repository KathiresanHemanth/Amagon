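; Assault rifle weapon Blueprint, a child of the weapon base that supplies the rifle's stats.
; BeginPlay runs the parent logic, then calls SetChildVar with hardcoded muzzle, range, reload, magazine, auto and burst timing, spread and bloom values.
; SetChildVar copies these into the weapon's variables and sets the current magazine to full capacity.
; It adds no firing logic of its own.
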(event EventBeginPlay
  (|CallParentFunction)
  (CallFunction|SetChildVar "Rifle" (Variables|Default|GetMullze%20Point_0) 5e+03 2.5 false 30 25 2 0.1 0.01 2.5 "/Game/_OWN/BP_PIckable/Equipments/Weapons/AR/BulletSpredCurve.BulletSpredCurve" 2.5))

(event Collision|EventActorBeginOverlap
  (params (OtherActor :type Actor%20Object%20Reference))
  (|CallParentFunction OtherActor) ; This node is disabled and will not be called.\nDrag off pins to build functionality.
)

(event EventTick
  (params (DeltaSeconds :type Float%20%28single-precision%29))
  (|CallParentFunction DeltaSeconds) ; This node is disabled and will not be called.\nDrag off pins to build functionality.
)

(fn ConstructionScript
  (|CallParentFunction))

(event Custom|Set%20child%20var
  (params (C%20Weapon%20type :type String) (Muzzle2 :type Static%20Mesh%20Component%20Object%20Reference) (C%20Range :type Float%20%28single-precision%29) (C%20Realod%20time :type Float%20%28single-precision%29) (C%20Infinty%20Ammo :type Boolean) (C%20Max%20Mag :type Integer) (C%20Spread%20Num%20of%20Bullets :type Integer) (C%20Burst%20Bullets%20Per%20tap%202 :type Integer) (C%20Time%20Between%20autoShooting :type Float%20%28single-precision%29) (C%20Time%20Between%20BurstShooting :type Float%20%28single-precision%29) (C%20Bloom%20Radius :type Float%20%28single-precision%29) (C%20Bloom%20curve :type Curve%20Float%20Object%20Reference) (C%20Bloom%20amount :type Float%20%28single-precision%29))
  (Variables|Default|SetC%20Weapon%20type C%20Weapon%20type)
  (Variables|Default|SetMuzzle Muzzle2)
  (Variables|Default|SetC%20Range C%20Range)
  (Variables|Default|SetC%20Realod%20time C%20Realod%20time)
  (Variables|Default|SetC%20Infinty%20Ammo C%20Infinty%20Ammo)
  (Variables|Default|SetD_Current%20Mag (Variables|Default|GetC%20Max%20Mag))
  (Variables|Default|SetC%20Max%20Mag C%20Max%20Mag)
  (Variables|Default|SetC%20Spread%20Num%20of%20Bullets C%20Spread%20Num%20of%20Bullets)
  (Variables|Default|SetC%20Burst%20Bullets%20Per%20tap%20 C%20Burst%20Bullets%20Per%20tap%202)
  (Variables|Default|SetC%20Time%20Between%20autoShooting C%20Time%20Between%20autoShooting)
  (Variables|Default|SetC%20Time%20Between%20BurstShooting C%20Time%20Between%20BurstShooting)
  (Variables|Default|SetC%20Bloom%20Radius C%20Bloom%20Radius)
  (Variables|Default|SetC%20Bloom%20curve C%20Bloom%20curve)
  (Variables|Default|SetC%20Bloom%20amount C%20Bloom%20amount))