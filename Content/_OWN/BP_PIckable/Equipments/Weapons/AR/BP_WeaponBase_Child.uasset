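; Child weapon Blueprint, filed under AR, that handles shooting, ammo use and timed reloading.
; Shoot spawns a bullet, sound and muzzle flash at the muzzle, plus a debug camera line trace whose hit is unused.
; AutoFire or a DoN-counted Burst loops back into that shot after a delay, while each shot also uses ammo or reloads.
; A separate Spread event draws randomized shotgun-style traces within a cone.
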(event Custom|Shoot
  (bind _returnvalue (Game|GetPlayerCameraManager 0))
  (bind _mullze_point_0 (Variables|Default|GetMullze%20Point_0))
  (bind _bullets_per_tap_0 (Variables|Mainpara|GetBullets%20Per%20tap_0))
  (bind _returnvalue_2 (Transformation|GetActorLocation _returnvalue))
  (bind _returnvalue_3 (Transformation|GetWorldLocation _mullze_point_0))
  ;[1 1 1] Shoot
  (Variables|Dynamic|SetD%20IsShooting_0 true)
  (Game|SpawnActorfromClass "/Game/_OWN/BP_PIckable/Equipments/Weapons/AR/BP_Bullete.BP_Bullete_C" (Math|Transform|MakeTransform _returnvalue_3 (Math|Rotator|MakeRotfromX (Math|Vector|GetForwardVector _mullze_point_0)) "0.200000,0.200000,0.200000") "Undefined" 0 0 :!label _label)
  (Audio|PlaySoundatLocation "/Game/_OWN/BP_PIckable/Equipments/Weapons/AR/Sfx/3GueSoundCue.3GueSoundCue" _returnvalue_3 "0, 0, 0" 1.0 1.0 0.0 0 0 0)
  (Effects|SpawnEmitterAttached "/Game/InfinityBladeEffects/Effects/FX_Monsters/FX_Monster_Chicken/P_ChickenMaster_MuzzleFlash_01.P_ChickenMaster_MuzzleFlash_01" _mullze_point_0 "None" "0, 0, 0" "0, 0, 0" "1.500000,1.500000,1.500000")
  (Collision|LineTraceByChannel _returnvalue_2 (+ _returnvalue_2 (* (Transformation|GetActorForwardVector _returnvalue) (Variables|Mainpara|GetRange_0))) "TraceTypeQuery1" true 0 "ForDuration" true "(R=1.000000,G=0.000000,B=0.000000,A=1.000000)" "(R=0.000000,G=1.000000,B=0.000000,A=1.000000)" 2e+01)
  (Utilities|FlowControl|Sequence
    (:then_0
      (if (Variables|Dynamic|GetD%20Full%20Auto?_0)
        (Utilities|AutoFire
          (:Completed
            (goto _label)))
        (elif (Variables|Dynamic|GetD%20Full%20Burst?_0)
          (bind _counter (Utilities|FlowControl|DoN _bullets_per_tap_0 :!label _label_2)
            (:Exit
              (CallFunction|Burst)
              (if (== _counter (- _bullets_per_tap_0 1))
                (Utilities|FlowControl|Delay 0.15)
                (goto _label_2 Reset)))))))
    (:then_1
      (if (and (!= (Variables|Dynamic|GetD_Current%20Mag_0) 0) (not (Variables|Dynamic|GetD%20Reloading?_0)))
        (CallFunction|UseAmmo)
        (else
          (CallFunction|Reload))))))

(event Custom|ReloadStart
  ;[1 1 1] Reload
  (if (!= (Variables|Dynamic|GetD_Ammo_0) 0)
    (Utilities|FlowControl|DoOnce false :!label _label
      (:Completed
        (Variables|Dynamic|SetD%20Reloading?_0 true)
        (Audio|PlaySoundatLocation "/Game/_OWN/BP_PIckable/Equipments/Weapons/AR/Sfx/Reload_Cue.Reload_Cue" (Transformation|GetActorLocation) "0, 0, 0" 2.0 1.0 0.0 0 0 0)
        (Utilities|FlowControl|Delay (Variables|Mainpara|GetRealod%20time_0))
        (CallFunction|Reload)
        (Variables|Dynamic|SetD%20Reloading?_0 false)
        (goto _label Reset)))))

(event Custom|Burst
  (bind _returnvalue (Game|GetPlayerCameraManager 0))
  (bind _mullze_point_0 (Variables|Default|GetMullze%20Point_0))
  (bind _bullets_per_tap_0 (Variables|Mainpara|GetBullets%20Per%20tap_0))
  (bind _returnvalue_2 (Transformation|GetActorLocation _returnvalue))
  (bind _returnvalue_3 (Transformation|GetWorldLocation _mullze_point_0))
  ;[1 1 1] Burst
  (if (and (!= (Variables|Dynamic|GetD_Current%20Mag_0) 0) (not (Variables|Dynamic|GetD%20Reloading?_0)))
    (Utilities|FlowControl|Delay (Variables|Mainpara|GetTime%20Between%20BurstShooting_0))
    ;[1 1 1] Shoot
    (Game|SpawnActorfromClass "/Game/_OWN/BP_PIckable/Equipments/Weapons/AR/BP_Bullete.BP_Bullete_C" (Math|Transform|MakeTransform _returnvalue_3 (Math|Rotator|MakeRotfromX (Math|Vector|GetForwardVector _mullze_point_0)) "0.200000,0.200000,0.200000") "Undefined" 0 0 :!label _label)
    (Audio|PlaySoundatLocation "/Game/_OWN/BP_PIckable/Equipments/Weapons/AR/Sfx/3GueSoundCue.3GueSoundCue" _returnvalue_3 "0, 0, 0" 1.0 1.0 0.0 0 0 0)
    (Effects|SpawnEmitterAttached "/Game/InfinityBladeEffects/Effects/FX_Monsters/FX_Monster_Chicken/P_ChickenMaster_MuzzleFlash_01.P_ChickenMaster_MuzzleFlash_01" _mullze_point_0 "None" "0, 0, 0" "0, 0, 0" "1.500000,1.500000,1.500000")
    (Collision|LineTraceByChannel _returnvalue_2 (+ _returnvalue_2 (* (Transformation|GetActorForwardVector _returnvalue) (Variables|Mainpara|GetRange_0))) "TraceTypeQuery1" true 0 "ForDuration" true "(R=1.000000,G=0.000000,B=0.000000,A=1.000000)" "(R=0.000000,G=1.000000,B=0.000000,A=1.000000)" 2e+01)
    (Utilities|FlowControl|Sequence
      (:then_0
        (if (Variables|Dynamic|GetD%20Full%20Auto?_0)
          (Utilities|AutoFire
            (:Completed
              (goto _label)))
          (elif (Variables|Dynamic|GetD%20Full%20Burst?_0)
            (bind _counter (Utilities|FlowControl|DoN _bullets_per_tap_0 :!label _label_2)
              (:Exit
                (CallFunction|Burst)
                (if (== _counter (- _bullets_per_tap_0 1))
                  (Utilities|FlowControl|Delay 0.15)
                  (goto _label_2 Reset)))))))
      (:then_1
        (if (and (!= (Variables|Dynamic|GetD_Current%20Mag_0) 0) (not (Variables|Dynamic|GetD%20Reloading?_0)))
          (CallFunction|UseAmmo)
          (else
            (CallFunction|Reload)))))))

(event Custom|Shoot%20realse
  ;[1 1 1] Realse Shoot
  (Variables|Dynamic|SetD%20IsShooting_0 false))

(event Custom|Spread
  (bind _returnvalue (Game|GetPlayerCameraManager 0))
  (bind _returnvalue_2 (Transformation|GetActorLocation _returnvalue))
  ;[1 1 1] Shot gun Spread
  (for _index (range 1 (Variables|Mainpara|GetNum%20of%20Bullets_0))
    (bind _point (CallFunction|RandPointinCircle (* (Math|Trig|Tan(Degrees) (Variables|Dynamic|GetD%20BulletAngle_0)) (Variables|Mainpara|GetRange_0))))
    (Collision|LineTraceByChannel _returnvalue_2 (+ (* (Transformation|GetActorForwardVector _returnvalue) (Variables|Mainpara|GetRange_0)) (* (Utilities|CameraRight) (.X (Math|Vector2D|BreakVector2D _point))) (* (Utilities|CameraUp) (.Y (Math|Vector2D|BreakVector2D _point))) _returnvalue_2) "TraceTypeQuery1" true (Utilities|Array|MakeArray (Game|Player|GetPlayerPawn 0)) "ForDuration" true "(R=1.000000,G=0.000000,B=0.000000,A=1.000000)" "(R=0.000000,G=1.000000,B=0.000000,A=1.000000)" 2e+01)))

(event EventBeginPlay
  (|CallParentFunction))

(event Collision|EventActorBeginOverlap
  (params (OtherActor :type Actor%20Object%20Reference))
  (|CallParentFunction OtherActor) ; This node is disabled and will not be called.\nDrag off pins to build functionality.
)

(event EventTick
  (params (DeltaSeconds :type Float%20%28single-precision%29))
  (|CallParentFunction DeltaSeconds) ; This node is disabled and will not be called.\nDrag off pins to build functionality.
)

(fn ConstructionScript
  (|CallParentFunction))