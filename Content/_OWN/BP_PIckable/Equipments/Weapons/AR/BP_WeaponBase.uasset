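; BP_WeaponBase is the base pickup weapon actor, whose construction script sets its skeletal mesh from a struct.
; An overlap sphere enables input for player 0 when a BP_Char_Gameplay enters and the weapon is not picked, and disables it one second after that character leaves.
; Pressing Pickup Object passes the weapon's class and actor to the character's EquipWP, then disables the weapon's input.
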(event OnComponentBeginOverlap(Sphere1)
  (params (OverlappedComponent :type Primitive%20Component%20Object%20Reference) (OtherActor :type Actor%20Object%20Reference) (OtherComp :type Primitive%20Component%20Object%20Reference) (OtherBodyIndex :type Integer) (bFromSweep :type Boolean) (SweepResult :type Hit%20Result%20Structure%20%28by%20ref%29))
  (if (not (Variables|Default|GetPicked))
    (bind _asbp_char_gameplay (Utilities|Casting|CastToBP_Char_Gameplay OtherActor))
    (Input|EnableInput (Game|GetPlayerController 0))))

(event OnComponentEndOverlap(Sphere1)
  (params (OverlappedComponent :type Primitive%20Component%20Object%20Reference) (OtherActor :type Actor%20Object%20Reference) (OtherComp :type Primitive%20Component%20Object%20Reference) (OtherBodyIndex :type Integer))
  (Utilities|Casting|CastToBP_Char_Gameplay OtherActor)
  (Utilities|FlowControl|Delay 1.0)
  (Input|DisableInput (Game|GetPlayerController 0)))

(event EventBeginPlay)

(event Collision|EventActorBeginOverlap
  (params (OtherActor :type Actor%20Object%20Reference)))

(event EventTick
  (params (DeltaSeconds :type Float%20%28single-precision%29)))

(event Input|ActionEvents|InputActionPickupObject
  (params (Key :type Key%20Structure :default "None"))
  (bind _self self)
  (:Pressed
    (Default|EquipWP (stale OnComponentBeginOverlap(Sphere1) _asbp_char_gameplay) (Utilities|GetClass _self) _self)
    (Input|DisableInput (Game|GetPlayerController 0))))

(fn ConstructionScript
  (Class|SkinnedMeshComponent|SetSkeletalMesh (Variables|Default|GetSkeletalMesh) (.skeleton (Variables|Default|GetStruct)) true))