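; Lobby player controller that shows a match stats widget and keeps its player count current.
; Creatematchwindow creates the widget with this controller as owner, stores it and adds it to the viewport.
; UpdatePlayerCount writes the received count into that widget if it is valid.
; An unconnected leftover would call CreateMatchWindow on the main menu game instance, but it never runs.
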(event Custom|Create%20match%20window
  (bind _returnvalue (UserInterface|CreateWidget "/Game/_OWN/UI/UI_Gameplay/LobbyMatchStats.LobbyMatchStats_C" self))
  (bind _output_get (Variables|Default|SetW/B%20Match%20Stats _returnvalue))
  (UserInterface|Viewport|AddtoViewport _output_get 0))

(event Custom|Update%20Player%20Count
  (params (Player%20Count :type String))
  (bind _w_b_match_stats (Variables|Default|GetW/B%20Match%20Stats))
  (Utilities|IsValid _w_b_match_stats
    (:Is%20Valid
      (Variables|/Game/_OWN/UI/UI_Gameplay/LobbyMatchStats.LobbyMatchStats_C|SetPlayer%20CountD _w_b_match_stats Player%20Count))))

(fn ConstructionScript)