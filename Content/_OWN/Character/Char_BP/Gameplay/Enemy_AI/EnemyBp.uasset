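; EnemyBp is an enemy AI character that chases the player.
; On BeginPlay it casts the player character to BP_Char_Gameplay, stores it and starts ChasePlayer with it as the target.
; ChasePlayer calls AI MoveTo on the player and, on success or failure, waits briefly and calls itself again, forming an endless chase loop.
; A randomized walk speed selection is present but disconnected, so it never runs.
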(event Custom|Chase%20Player
  (params (Player :type BP%20Char%20Gameplay%20Object%20Reference))
  (AI|AIMoveTo self "0, 0, 0" Player 5.0 false
    (:OnSuccess
      _)
    (:OnFail
      _))
  (Utilities|FlowControl|Delay 2.0)
  (CallFunction|ChasePlayer (Variables|Default|GetChar%20ref)))

(event EventBeginPlay
  (bind _asbp_char_gameplay (Utilities|Casting|CastToBP_Char_Gameplay (Game|GetPlayerCharacter 0)))
  (bind _output_get (Variables|Default|SetChar%20ref _asbp_char_gameplay))
  (CallFunction|ChasePlayer _output_get))

(fn ConstructionScript)