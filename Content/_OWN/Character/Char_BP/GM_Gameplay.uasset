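; GM_Gameplay is the gameplay GameMode, managing joining players, the match player count and pawn spawning.
; PostLogin registers each controller, opens its match window, then after short delays pushes the player count and team value to all PC_Gameplay controllers.
; BeginPlay spawns and possesses a character for player 0 at a random PlayerStart, whose index doubles as the team value.
; Logout calls session destruction on MainmenuGameInstance, removes the controller and refreshes the count.
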(event Custom|Update%20players
  ;[1 1 1] Update Player for Auto match
  (Utilities|FlowControl|Delay 0.6)
  (bind _asmainmenu_game_instance (Utilities|Casting|CastToMainmenuGameInstance (Game|GetGameInstance)))
  (for _array_element (Variables|Default|GetAll%20Player%20Controllers)
    (bind _aspc_gameplay (Utilities|Casting|CastToPC_Gameplay _array_element))
    (Default|UpdatePlayerCount _aspc_gameplay (Utilities|String|Append (Utilities|String|ToString(Integer) (Utilities|Array|Length (Variables|Default|GetAll%20Player%20Controllers))) "/" (Utilities|String|ToString(Integer) (Variables|/Game/_OWN/UI/Mainmenu_UI/BP/MainmenuGameInstance.MainmenuGameInstance_C|GetV%20Max%20Players _asmainmenu_game_instance))))))

(event Custom|Respawn%20Player
  (params (Player%20Controller :type Player%20Controller%20Object%20Reference) (Player%20Character :type Character%20Class%20Reference))
  (bind _returnvalue (Pawn|GetControlledPawn Player%20Controller))
  ;[1 1 1] Spawn the Player With the Selected character
  (bind _outactors (Actor|GetAllActorsOfClass "/Script/Engine.PlayerStart"))
  (Variables|Default|SetSpawn%20Points _outactors)
  (Utilities|IsValid _returnvalue
    (:Is%20Valid
      (Actor|DestroyActor _returnvalue))
    (:Is%20Not%20Valid
      _))
  (Variables|Default|SetGet%20Team%20 (.OutIndex (Utilities|Array|Random (Variables|Default|GetSpawn%20Points))))
  (bind _returnvalue_2 (Game|SpawnActorfromClass Player%20Character (Transformation|GetActorTransform (Utilities|Array|Get(acopy) (Variables|Default|GetSpawn%20Points) (Variables|Default|GetGet%20Team%20))) "Undefined" 0 0))
  (Pawn|Possess Player%20Controller _returnvalue_2))

(event Custom|Updates%20team
  (bind _all_player_controllers (Variables|Default|GetAll%20Player%20Controllers))
  (Utilities|FlowControl|Delay 0.6)
  (Development|PrintString (Utilities|String|ToString(Integer) (Utilities|Array|Length _all_player_controllers)) true true "(R=0.000000,G=0.660000,B=1.000000,A=1.000000)" 1e+01)
  (for _array_element _all_player_controllers
    (bind _aspc_gameplay (Utilities|Casting|CastToPC_Gameplay _array_element))
    (Default|UpdateTeam _aspc_gameplay (Variables|Default|GetGet%20Team%20))))

(event EventPostLogin
  (params (NewPlayer :type Player%20Controller%20Object%20Reference))
  (Networking|SwitchHasAuthority
    (:Authority
      (Utilities|Array|Add (Variables|Default|GetAll%20Player%20Controllers) NewPlayer)
      (bind _aspc_gameplay (Utilities|Casting|CastToPC_Gameplay NewPlayer)
        (:then
          (Default|CreateMatchWindow _aspc_gameplay)
          (CallFunction|UpdatePlayers)
          (CallFunction|UpdatesTeam))
        (:CastFailed
          (Development|PrintString "Cast Failef"))))))

(event EventBeginPlay
  ;[1 1 1] Event Begin
  (CallFunction|RespawnPlayer (Game|GetPlayerController 0) "/Game/_OWN/Character/Char_BP/BP_Char_Gameplay.BP_Char_Gameplay_C"))

(event EventOnLogout
  (params (ExitingController :type Controller%20Object%20Reference))
  ;[1 1 1] ON Logout , Destroy session
  (bind _aspc_gameplay (Utilities|Casting|CastToPC_Gameplay ExitingController))
  (Default|DestroySessionCaller (.AsMainmenu%20Game%20Instance (Utilities|Casting|CastToMainmenuGameInstance (Game|GetGameInstance))) _aspc_gameplay)
  ;[1 1 1] On Logout
  (bind (_array_element _array_index) (Utilities|Array|ForEachLoopwithBreak (Variables|Default|GetAll%20Player%20Controllers) :!label _label)
    (:LoopBody
      (if (== 0 _array_element)
        (goto _label Break)))
    (:Completed
      ;[1 1 1] Remove From Array
      (Utilities|Array|RemoveIndex (Variables|Default|GetAll%20Player%20Controllers) _array_index)
      (CallFunction|UpdatePlayers))))

(fn ConstructionScript)