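; Lobby GameMode that tracks joining and leaving players and decides when the match can start.
; On login it stores the controller, opens its match window and reads the "Server Name" session setting to flag auto-generated matches.
; Delayed updates send player counts to each PC_Lobby and compare them to a fraction of max capacity.
; At that threshold, auto matches server-travel to GameplayMenu, while custom rooms enable the room widget's Start button.
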(event Custom|Update%20players
  (Utilities|FlowControl|Delay 0.6)
  (bind _asmainmenu_game_instance (Utilities|Casting|CastToMainmenuGameInstance (Game|GetGameInstance)))
  ;[1 1 1] Update Player for Auto match
  (if (Variables|Default|GetIS%20auto%20generated)
    (for _array_element (Variables|Default|GetAll%20Player%20Controllers)
      (bind _aspc_lobby (Utilities|Casting|CastToPC_Lobby _array_element))
      (Default|UpdatePlayerCount _aspc_lobby (Utilities|String|Append (Utilities|String|ToString(Integer) (Utilities|Array|Length (Variables|Default|GetAll%20Player%20Controllers))) "/" (Utilities|String|ToString(Integer) (Variables|/Game/_OWN/UI/Mainmenu_UI/BP/MainmenuGameInstance.MainmenuGameInstance_C|GetV%20Max%20Players _asmainmenu_game_instance)))))
    (if (>= (Utilities|Array|Length (Variables|Default|GetAll%20Player%20Controllers)) (Math|Float|Round (/ (Math|Conversions|ToFloat(Integer) (Variables|/Game/_OWN/UI/Mainmenu_UI/BP/MainmenuGameInstance.MainmenuGameInstance_C|GetV%20Max%20Players _asmainmenu_game_instance)) (Variables|Default|GetDivide%20Float))))
      (Development|PrintString "Ok to Start")
      (Utilities|FlowControl|Delay 2.0)
      (CallFunction|LaunchGame)
      (else
        (Development|PrintString "waiting")))
    (else
      ;[1 1 1] Update Player Count
      (Variables|/Game/_OWN/UI/Mainmenu_UI/BP/ShowRoomDetail.ShowRoomDetail_C|SetPLayer%20in%20room (Variables|/Game/_OWN/UI/Mainmenu_UI/BP/MainmenuGameInstance.MainmenuGameInstance_C|GetW/b%20Show%20Room%20Detail%20REF _asmainmenu_game_instance) (Utilities|String|Append (Utilities|String|ToString(Integer) (Utilities|Array|Length (Variables|Default|GetAll%20Player%20Controllers))) "/" (Utilities|String|ToString(Integer) (Variables|/Game/_OWN/UI/Mainmenu_UI/BP/MainmenuGameInstance.MainmenuGameInstance_C|GetRoom%20Max%20Num%20Player _asmainmenu_game_instance))))
      (for _array_element_2 (Variables|Default|GetAll%20Player%20Controllers)
        (bind _aspc_lobby_2 (Utilities|Casting|CastToPC_Lobby _array_element_2))
        (Default|UpdatePlayerCount _aspc_lobby_2 (Utilities|String|Append (Utilities|String|ToString(Integer) (Utilities|Array|Length (Variables|Default|GetAll%20Player%20Controllers))) "/" (Utilities|String|ToString(Integer) (Variables|/Game/_OWN/UI/Mainmenu_UI/BP/MainmenuGameInstance.MainmenuGameInstance_C|GetRoom%20Max%20Num%20Player _asmainmenu_game_instance)))))
      ;[1 1 1] Set Start Button
      (if (>= (Utilities|Array|Length (Variables|Default|GetAll%20Player%20Controllers)) (Math|Float|Round (/ (Math|Conversions|ToFloat(Integer) (Variables|/Game/_OWN/UI/Mainmenu_UI/BP/MainmenuGameInstance.MainmenuGameInstance_C|GetRoom%20Max%20Num%20Player _asmainmenu_game_instance)) (Variables|Default|GetDivide%20Float))))
        (Development|PrintString "Ok to Start")
        (bind _asmainmenu_game_instance_2 (Utilities|Casting|CastToMainmenuGameInstance (Game|GetGameInstance)))
        (Widget|SetIsEnabled (Variables|/Game/_OWN/UI/Mainmenu_UI/BP/ShowRoomDetail.ShowRoomDetail_C|GetStart (Variables|/Game/_OWN/UI/Mainmenu_UI/BP/MainmenuGameInstance.MainmenuGameInstance_C|GetW/b%20Show%20Room%20Detail%20REF _asmainmenu_game_instance_2)) true)
        (else
          (Development|PrintString "waiting")
          (bind _asmainmenu_game_instance_3 (Utilities|Casting|CastToMainmenuGameInstance (Game|GetGameInstance)))
          (Widget|SetIsEnabled (Variables|/Game/_OWN/UI/Mainmenu_UI/BP/ShowRoomDetail.ShowRoomDetail_C|GetStart (Variables|/Game/_OWN/UI/Mainmenu_UI/BP/MainmenuGameInstance.MainmenuGameInstance_C|GetW/b%20Show%20Room%20Detail%20REF _asmainmenu_game_instance_3)) false))))))

(event Custom|Launch%20Game
  (Development|ExecuteConsoleCommand (Utilities|String|Append "servertravel " "/Game/_OWN/Level/" "GameplayMenu") (Game|GetPlayerController 0)))

(event EventPostLogin
  (params (NewPlayer :type Player%20Controller%20Object%20Reference))
  ;[1 1 1] Event on login
  (Networking|SwitchHasAuthority
    (:Authority
      (Utilities|Array|Add (Variables|Default|GetAll%20Player%20Controllers) NewPlayer)
      (bind _aspc_lobby (Utilities|Casting|CastToPC_Lobby NewPlayer))
      (Default|CreateMatchWindow _aspc_lobby)
      (bind _extrasettings (Class|AdvancedSessionsLibrary|GetSessionSettings)
        (:OnSuccess
          (bind _settingvalue (Class|AdvancedSessionsLibrary|GetSessionPropertyString _extrasettings "Server Name")
            (:Found
              (Variables|Default|SetIS%20auto%20generated (Utilities|Enum|Equal(Enum) _settingvalue "Auto"))
              (CallFunction|UpdatePlayers))))))))

(event EventOnLogout
  (params (ExitingController :type Controller%20Object%20Reference))
  ;[1 1 1] On Logout
  (bind (_array_element _array_index) (Utilities|Array|ForEachLoopwithBreak (Variables|Default|GetAll%20Player%20Controllers) :!label _label)
    (:LoopBody
      (if (== ExitingController _array_element)
        (goto _label Break)))
    (:Completed
      ;[1 1 1] Remove From Array
      (Utilities|Array|RemoveIndex (Variables|Default|GetAll%20Player%20Controllers) _array_index)
      (CallFunction|UpdatePlayers))))

(fn ConstructionScript)