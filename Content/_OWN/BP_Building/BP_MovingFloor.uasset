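; Moving floor actor that wanders endlessly through random positions, starting at BeginPlay.
; Each move picks a random offset from the current location within ZMax, with half that range horizontally.
; The Move timeline lerps the actor there with sweep enabled, scaling its track by ten for the alpha, then triggers the next move when finished.
; Offsets accumulate from wherever it stops, so it is not bound to its spawn point.
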(event Custom|Move%20Building
  (bind _z_max (Variables|Default|GetZ%20Max))
  (bind _returnvalue (/ _z_max 2.0))
  (bind _returnvalue_2 (Class|TKMathFunctionLibrary|NegateFloat _returnvalue))
  (Variables|Default|SetStart%20Location (Transformation|GetActorLocation))
  (Variables|Default|SetNew%20Location (+ (Transformation|GetActorLocation) (Math|Vector|MakeVector (Math|Random|RandomFloatinRange _returnvalue_2 _returnvalue) (Math|Random|RandomFloatinRange _returnvalue_2 _returnvalue) (Math|Random|RandomFloatinRange (Class|TKMathFunctionLibrary|NegateFloat _z_max) _z_max))))
  (bind _newtrack_0 (Timeline|Move PlayFromStart)
    (:Update
      (Transformation|SetActorLocation (Math|Vector|Lerp(Vector) (Variables|Default|GetStart%20Location) (+ (Variables|Default|GetNew%20Location) "0, 0, 0") (* _newtrack_0 1e+01)) true false))
    (:Finished
      (CallFunction|MoveBuilding))))

(event EventBeginPlay
  (CallFunction|MoveBuilding))

(fn ConstructionScript)